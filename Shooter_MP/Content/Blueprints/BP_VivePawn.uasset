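; Multiplayer VR pawn for Vive that replicates head and hand transforms and colors the right hand while its trigger is held.
; Each tick it reads motion controller poses if locally controlled, then sends them with the camera transform through a server update event.
; OnRep functions apply hand transforms to the hand components.
; Trigger input swaps yellow and blue materials through a server event; the trigger's OnRep is empty.
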(event `self.ReceiveTick`
  (params (DeltaSeconds :type "Float (single-precision)"))
  ;[1 1 1] Update transforms locally
  (`self.UpdateHandTransformsLocal`)
  (`self.ServerUpdateTransforms` (`self.LeftHandTransform`) (`self.RightHandTransform`) (`SceneComponent.GetRelativeTransform` (`self.Camera`))))

(event `ServerUpdateTransforms`
  (params (`Left Hand` :type "Transform Structure") (`Right Hand` :type "Transform Structure") (Head :type "Transform Structure"))
  ;[1 1 1] Update transforms on server
  (set `self.LeftHandTransform` `Left Hand`)
  (set `self.RightHandTransform` `Right Hand`)
  (`SceneComponent.K2_SetRelativeTransform` (`self.Camera`) Head false false))

(event `Key|MotionController_Right_Trigger`
  (params (Key :type "Key Structure" :default "AnyKey"))
  (:`Pressed`
    (bind _output_get (set `self.RightTriggerPressed` true))
    (`self.ServerUpdateHandColor` _output_get))
  (:`Released`
    (bind _output_get_2 (set `self.RightTriggerPressed` false))
    (`self.ServerUpdateHandColor` _output_get_2)))

(event `ServerUpdateHandColor`
  (params (RightTriggerPressed :type Boolean))
  (bind _righthand (`self.RightHand`))
  (if RightTriggerPressed
    (`PrimitiveComponent.SetMaterial` _righthand 0 "/Game/Materials/M_Yellow.M_Yellow")
    (else
      (`PrimitiveComponent.SetMaterial` _righthand 0 "/Game/Materials/M_Blue.M_Blue"))))

(fn `OnRep_LeftHandTransform`
  (`SceneComponent.K2_SetRelativeTransform` (`self.LeftHand`) (`self.LeftHandTransform`) false false))

(fn `OnRep_RightHandTransform`
  (`SceneComponent.K2_SetRelativeTransform` (`self.RightHand`) (`self.RightHandTransform`) false false))

(fn `OnRep_RightTriggerPressed`)

(fn `UpdateHandTransformsLocal`
  (bind (_outposition _outorientation) (`SteamVRFunctionLibrary.GetHandPositionAndOrientation` 0 "Right"))
  (bind (_outposition_2 _outorientation_2) (`SteamVRFunctionLibrary.GetHandPositionAndOrientation` 0 "Left"))
  (if (`self.IsLocallyControlled`)
    (set `self.LeftHandTransform` (`KismetMathLibrary.MakeTransform` _outposition_2 _outorientation_2 (0.2 0.2 0.2)))
    (set `self.RightHandTransform` (`KismetMathLibrary.MakeTransform` _outposition _outorientation (0.2 0.2 0.2)))))

(fn `UserConstructionScript`)