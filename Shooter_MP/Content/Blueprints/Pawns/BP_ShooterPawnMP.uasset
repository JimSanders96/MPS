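; Multiplayer VR shooter pawn with tracked hands and a right-hand gun fired by the motion controller trigger.
; Each tick it reads controller poses when locally controlled and sends hand and head transforms through a server event.
; OnRep handlers apply the hand transforms, while the server event sets the camera transform directly.
; The trigger calls Fire on the child-actor gun; the pressed-state hand color is incomplete, since setting it true is unwired.
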(event `self.ReceiveBeginPlay`
  (bind _asbp_gun_mp (cast `/Game/Blueprints/Usables/Guns/BP_GunMP` (`ChildActorComponent.ChildActor` (`self.RightHandGun`))))
  (set `/Game/Blueprints/Usables/Guns/BP_GunMP.OwningPlayer` self _asbp_gun_mp)
  (set `self.RightHandGunBP` _asbp_gun_mp))

(event `self.ReceiveTick`
  (params (DeltaSeconds :type "Float (single-precision)"))
  ;[1 1 1] Update transforms locally
  (`self.UpdateHandTransformsLocal`)
  (`self.ServerUpdateTransforms` (`self.LeftHandTransform`) (`self.RightHandTransform`) (`SceneComponent.GetRelativeTransform` (`self.Camera`))))

(event `ServerUpdateTransforms`
  (params (`Left Hand` :type "Transform Structure") (`Right Hand` :type "Transform Structure") (Head :type "Transform Structure"))
  ;[1 1 1] Update transforms on server
  (set `self.LeftHandTransform` `Left Hand`)
  (set `self.RightHandTransform` `Right Hand`)
  (`SceneComponent.K2_SetRelativeTransform` (`self.Camera`) Head false false))

(event `Key|MotionController_Right_Trigger`
  (params (Key :type "Key Structure" :default "AnyKey"))
  (:`Pressed`
    (`self.FireRightWeapon`))
  (:`Released`
    (set `self.RightTriggerPressed` false)))

(event `FireRightWeapon`
  (`/Game/Blueprints/Usables/Guns/BP_GunMP.Fire` (`self.RightHandGunBP`)))

(fn `OnRep_LeftHandTransform`
  ;[1 1 1] Only set the new transform for other players than yourself. Yours is already updated locally
  (`SceneComponent.K2_SetRelativeTransform` (`self.LeftHand`) (`self.LeftHandTransform`) false false))

(fn `OnRep_RightHandTransform`
  ;[1 1 1] Only set the new transform for other players than yourself. Yours is already updated locally
  (`SceneComponent.K2_SetRelativeTransform` (`self.RightHand`) (`self.RightHandTransform`) false false))

(fn `OnRep_RightTriggerPressed`
  (if (`self.RightTriggerPressed`)
    (`PrimitiveComponent.SetMaterial` (`self.RightHand`) 0 "/Game/Materials/Basic/M_Yellow.M_Yellow")
    (else
      (`PrimitiveComponent.SetMaterial` (`self.RightHand`) 0 "/Game/Materials/Basic/M_Blue.M_Blue"))))

(fn `UpdateHandTransformsLocal`
  (bind (_outposition _outorientation) (`SteamVRFunctionLibrary.GetHandPositionAndOrientation` 0 "Right"))
  (bind (_outposition_2 _outorientation_2) (`SteamVRFunctionLibrary.GetHandPositionAndOrientation` 0 "Left"))
  ;[1 1 1] Get the location and rotation of the controllers and store them in the replicated transforms
  (if (`self.IsLocallyControlled`)
    (set `self.LeftHandTransform` (`KismetMathLibrary.MakeTransform` _outposition_2 _outorientation_2 (`self.HandScale`)))
    (set `self.RightHandTransform` (`KismetMathLibrary.MakeTransform` _outposition _outorientation (`self.HandScale`)))))

(fn `UserConstructionScript`)