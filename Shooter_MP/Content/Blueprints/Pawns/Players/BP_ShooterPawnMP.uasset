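; Multiplayer VR shooter pawn with a gun in the right hand and an object pickup handler in the left.
; The locally controlled pawn reads controller poses each Tick, and ServerUpdateTransforms passes hand and camera transforms to the server.
; OnRep functions apply the replicated hand transforms to the hand components.
; Right trigger fires the gun child actor; left trigger press and release drive pickup and drop through the handler child actor.
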(event `self.ReceiveBeginPlay`
  ;[1 1 1] Get and set the right hand gun reference
  (bind _asbp_gun_mp (cast `/Game/Blueprints/Usables/Guns/BP_GunMP` (`ChildActorComponent.ChildActor` (`self.RightHandGun`))))
  (set `self.RightHandGunBP` _asbp_gun_mp)
  ;[1 1 1] Get and set the left hand pickup handler reference
  (bind _asbp_object_pickup_handler (cast `/Game/Blueprints/Usables/BP_ObjectPickupHandler` (`ChildActorComponent.ChildActor` (`self.LeftHandPickupHandler`))))
  (set `self.LHPickupHandlerBP` _asbp_object_pickup_handler))

(event `ServerUpdateTransforms`
  (params (`Left Hand` :type "Transform Structure") (`Right Hand` :type "Transform Structure") (Head :type "Transform Structure"))
  ;[1 1 1] Update transforms on server
  (set `self.LeftHandTransform` `Left Hand`)
  (set `self.RightHandTransform` `Right Hand`)
  (`SceneComponent.K2_SetRelativeTransform` (`self.Camera`) Head false false))

(event `self.ReceiveTick`
  (params (DeltaSeconds :type "Float (single-precision)"))
  ;[1 1 1] Update transforms locally
  (`self.UpdateHandTransformsLocal`)
  (`self.ServerUpdateTransforms` (`self.LeftHandTransform`) (`self.RightHandTransform`) (`SceneComponent.GetRelativeTransform` (`self.Camera`))))

(event `Key|MotionController_Right_Trigger`
  (params (Key :type "Key Structure" :default "AnyKey"))
  ;[1 1 1] Fire the weapon when the right trigger is pressed
  (:`Pressed`
    (`self.FireRightWeapon`)))

(event `Key|MotionController_Left_Trigger`
  (params (Key :type "Key Structure" :default "AnyKey"))
  ;[1 1 1] When left trigger is pressed, pick up the detected item
  (:`Pressed`
    (`self.PickupWithLeftHand`))
  (:`Released`
    ;[1 1 1] When left trigger is released, release the picked up item
    (`self.ReleaseWithLeftHand`)))

(event `PickupWithLeftHand`
  ;[1 1 1] Pickup with left hand
  (`/Game/Blueprints/Usables/BP_ObjectPickupHandler.PickUp` (`self.LHPickupHandlerBP`)))

(event `ReleaseWithLeftHand`
  ;[1 1 1] Release with left hand
  (`/Game/Blueprints/Usables/BP_ObjectPickupHandler.Release` (`self.LHPickupHandlerBP`)))

(event `FireRightWeapon`
  ;[1 1 1] Fire right weapon
  (`/Game/Blueprints/Usables/Guns/BP_GunMP.Fire` (`self.RightHandGunBP`)))

(fn `OnRep_LeftHandTransform`
  (`SceneComponent.K2_SetRelativeTransform` (`self.LeftHand`) (`self.LeftHandTransform`) false false))

(fn `OnRep_RightHandTransform`
  ;[1 1 1] Only set the new transform for other players than yourself. Yours is already updated locally
  (`SceneComponent.K2_SetRelativeTransform` (`self.RightHand`) (`self.RightHandTransform`) false false))

(fn `UpdateHandTransformsLocal`
  (bind (_outposition _outorientation) (`SteamVRFunctionLibrary.GetHandPositionAndOrientation` 0 "Right"))
  (bind (_outposition_2 _outorientation_2) (`SteamVRFunctionLibrary.GetHandPositionAndOrientation` 0 "Left"))
  ;[1 1 1] Get the location and rotation of the controllers and store them in the replicated transforms
  (if (`self.IsLocallyControlled`)
    (set `self.LeftHandTransform` (`KismetMathLibrary.MakeTransform` _outposition_2 _outorientation_2 (`self.HandScale`)))
    (set `self.RightHandTransform` (`KismetMathLibrary.MakeTransform` _outposition _outorientation (`self.HandScale`)))))

(fn `UserConstructionScript`)