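; BP_PhysicsObjectMP is a multiplayer physics cube that simulates only on the server.
; The server writes the cube's world transform to a replicated variable every tick.
; Clients disable physics, store each replicated transform through its OnRep, and lerp halfway toward it every tick, so smoothing depends on frame rate.
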(event `self.ReceiveBeginPlay`
  ;[1 1 1] Determine whether this instance of the cube is on the server or not for future reference
  (bind _output_get (set `self.OnServer` (`KismetSystemLibrary.IsServer`)))
  ;[1 1 1] If the cube isn't on the server, don't simulate physics
  (if (not _output_get)
    (`PrimitiveComponent.SetSimulatePhysics` (`self.Cube`) false)))

(event `self.ReceiveTick`
  (params (DeltaSeconds :type "Float (single-precision)"))
  (bind _cube (`self.Cube`))
  ;[1 1 1] Update CubeTransform on server only
  (if (`self.OnServer`)
    (set `self.ObjectTransform` (`SceneComponent.K2_GetComponentToWorld` (`self.Cube`)))
    (else
      ;[1 1 1] Smoothly update the transform on clients
      (`SceneComponent.K2_SetWorldTransform` _cube (`KismetMathLibrary.TLerp` (`SceneComponent.K2_GetComponentToWorld` _cube) (`self.LatestTransform`) 0.5) false false))))

(fn `OnRep_CubeTransform`
  ;[1 1 1] Update the transform only if this isn't the server
  (if (not (`self.OnServer`))
    (set `self.LatestTransform` (`self.ObjectTransform`))))

(fn `UserConstructionScript`)