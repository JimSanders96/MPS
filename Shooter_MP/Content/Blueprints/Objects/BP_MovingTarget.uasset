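; BP_MovingTarget is a target actor meant to travel vertically between destination points, with the initial destination set on the server at BeginPlay.
; ResetDestination offsets Destination Z by StraightDistance according to MovingUp, but both branches set MovingUp true.
; MoveToDestination loops, stepping the root by Speed and testing Destination, rather than actor location, against min/max bounds.
; Nothing here calls MoveToDestination, and the bounds calculation is unconnected.
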(event `self.ReceiveBeginPlay`
  (`/Engine/EditorBlueprintResources/ActorMacros.Switch Has Authority`
    (:`Authority`
      (`self.ResetDestination`))))

(event `ResetDestination`
  (bind (_destination_x _destination_y _destination_z) (`KismetMathLibrary.BreakVector` (`self.Destination`)))
  (bind (_destination_x_2 _destination_y_2 _destination_z_2) (`KismetMathLibrary.BreakVector` (`self.Destination`)))
  ;[1 1 1] Reset destination
  (set `self.DestinationReached` true)
  (if (`self.MovingUp`)
    (set `self.Destination` (`KismetMathLibrary.MakeVector` _destination_x _destination_y (- _destination_z (`self.StraightDistance`))))
    (set `self.MovingUp` true)
    (else
      (set `self.Destination` (`KismetMathLibrary.MakeVector` _destination_x_2 _destination_y_2 (+ _destination_z_2 (`self.StraightDistance`))))
      (set `self.MovingUp` true)))
  (set `self.DestinationReached` false))

(event `MoveToDestination`
  (bind _defaultsceneroot (`self.DefaultSceneRoot`))
  (bind _defaultsceneroot_2 (`self.DefaultSceneRoot`))
  (bind (_destination_x _destination_y _destination_z) (`KismetMathLibrary.BreakVector` (`self.Destination`)))
  (bind (_destinationmin_x _destinationmin_y _destinationmin_z) (`KismetMathLibrary.BreakVector` (`self.DestinationMin`)))
  (bind (_destination_x_2 _destination_y_2 _destination_z_2) (`KismetMathLibrary.BreakVector` (`self.Destination`)))
  (bind (_destinationmax_x _destinationmax_y _destinationmax_z) (`KismetMathLibrary.BreakVector` (`self.DestinationMax`)))
  (bind (_returnvalue_x _returnvalue_y _returnvalue_z) (`KismetMathLibrary.BreakVector` (`SceneComponent.K2_GetComponentLocation` _defaultsceneroot)))
  (bind (_returnvalue_x_2 _returnvalue_y_2 _returnvalue_z_2) (`KismetMathLibrary.BreakVector` (`SceneComponent.K2_GetComponentLocation` _defaultsceneroot_2)))
  (while (not (`self.DestinationReached`))
    (if (`self.MovingUp`)
      (`SceneComponent.K2_SetWorldLocation` _defaultsceneroot_2 (`KismetMathLibrary.MakeVector` _returnvalue_x_2 _returnvalue_y_2 (+ _returnvalue_z_2 (`self.Speed`))) false false)
      (else
        (`SceneComponent.K2_SetWorldLocation` _defaultsceneroot (`KismetMathLibrary.MakeVector` _returnvalue_x _returnvalue_y (- _returnvalue_z (`self.Speed`))) false false)))
    (if (>= _destination_z _destinationmin_z)
      (if (<= _destination_z_2 _destinationmax_z)
        (`self.ResetDestination`)))))

(fn `UserConstructionScript`
  (`parent.UserConstructionScript`))