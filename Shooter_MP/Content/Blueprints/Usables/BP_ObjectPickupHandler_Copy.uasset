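; Server-authoritative pickup handler that lets physics objects be grabbed, carried and thrown.
; A sphere overlap tracks the nearby BP_PhysicsObjectBase as the detected object.
; PickUp disables that object's physics and attaches it, then Tick teleports its cube to the sphere's transform, preserving scale.
; ReleaseEvent stops the snapping and calls Release, which detaches the object, re-enables physics and applies the throw impulse.
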(event `self.ReceiveTick`
  (params (DeltaSeconds :type "Float (single-precision)"))
  (`/Engine/EditorBlueprintResources/ActorMacros.Switch Has Authority`
    (:`Authority`
      (if (`self.ObjectPickedUp`)
        ;[1 1 1] Snap object
        (`SceneComponent.K2_SetWorldTransform` (`/Game/Blueprints/Objects/BP_PhysicsObjectBase.Cube` (`self.PickedUpObject`)) (`KismetMathLibrary.MakeTransform` (.location (`SceneComponent.K2_GetComponentToWorld` (`self.Sphere`))) (.rotation (`SceneComponent.K2_GetComponentToWorld` (`self.Sphere`))) (`self.PickedUpObjectScale`)) false false)))))

(event `self.Sphere.OnComponentBeginOverlap`
  (params (OverlappedComponent :type "PrimitiveComponent Object Reference") (OtherActor :type "Actor Object Reference") (OtherComp :type "PrimitiveComponent Object Reference") (OtherBodyIndex :type Integer) (bFromSweep :type Boolean) (SweepResult :type "HitResult Structure (by ref)"))
  ;[1 1 1] Detect objects
  (`/Engine/EditorBlueprintResources/ActorMacros.Switch Has Authority`
    (:`Authority`
      (bind _asbp_physics_object_base (cast `/Game/Blueprints/Objects/BP_PhysicsObjectBase` OtherActor))
      (set `self.DetectedObject` _asbp_physics_object_base))))

(event `self.Sphere.OnComponentEndOverlap`
  (params (OverlappedComponent :type "PrimitiveComponent Object Reference") (OtherActor :type "Actor Object Reference") (OtherComp :type "PrimitiveComponent Object Reference") (OtherBodyIndex :type Integer))
  ;[1 1 1] Detect objects
  (`/Engine/EditorBlueprintResources/ActorMacros.Switch Has Authority`
    (:`Authority`
      (bind _asbp_physics_object_base (cast `/Game/Blueprints/Objects/BP_PhysicsObjectBase` OtherActor))
      (if (== _asbp_physics_object_base (`self.DetectedObject`))
        (set `self.DetectedObject` null)))))

(event `ReleaseEvent`
  (params (ThrowForce :type "Vector Structure"))
  (set `self.ObjectPickedUp` false)
  (`self.Release` ThrowForce))

(fn `PickUp`
  (`/Engine/EditorBlueprintResources/ActorMacros.Switch Has Authority`
    (:`Authority`
      (if (!= (`self.DetectedObject`) null)
        (bind _output_get (set `self.PickedUpObject` (`self.DetectedObject`)))
        (bind _cube (`/Game/Blueprints/Objects/BP_PhysicsObjectBase.Cube` _output_get))
        (`PrimitiveComponent.SetSimulatePhysics` _cube false)
        (`self.K2_AttachToComponent` _output_get (`self.DefaultSceneRoot`) "None" "SnapToTarget" "SnapToTarget" "KeepRelative" true)
        (bind (_returnvalue_location _returnvalue_rotation _returnvalue_scale) (`KismetMathLibrary.BreakTransform` (`SceneComponent.K2_GetComponentToWorld` _cube)))
        (set `self.PickedUpObjectScale` _returnvalue_scale)
        (set `self.ObjectPickedUp` true)))))

(fn `Release`
  (params (ThrowForce :type "Vector Structure"))
  (bind _pickedupobject (`self.PickedUpObject`))
  (bind _cube (`/Game/Blueprints/Objects/BP_PhysicsObjectBase.Cube` _pickedupobject))
  (`/Engine/EditorBlueprintResources/ActorMacros.Switch Has Authority`
    (:`Authority`
      (if (!= (`self.PickedUpObject`) null)
        (`self.K2_DetachFromActor` _pickedupobject "KeepRelative" "KeepRelative" "KeepRelative")
        (`PrimitiveComponent.SetSimulatePhysics` _cube true)
        (`PrimitiveComponent.AddImpulse` _cube ThrowForce "None" false)
        (set `self.PickedUpObject` null)))))

(fn `UserConstructionScript`)