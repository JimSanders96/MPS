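; VR archery pawn that holds a spawned bow in the left hand and spawns an arrow in the right on trigger press.
; Tick nocks the arrow when hands are close, then maps hand distance to string pull and haptics.
; Releasing the trigger shoots at distance-based speed or drops an unnocked arrow; a sustained pull charges a straight-flying super arrow with a larger hitbox.
; Two-hand mode toggle and trace-arrow preview are unwired.
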(event `self.ReceiveBeginPlay`
  ;[0 0.7608 1] spawns bow and attaches it to left hand
  (`self.BowSpawnAndAttachToLeftHand`))

(event `Key|MotionController_Right_Trigger`
  (params (Key :type "Key Structure" :default "AnyKey"))
  (:`Pressed`
    ;[0 0.7608 1] spawns arrow and attaches it to right hand
    (`self.ArrowSpawnAndAttachToRightHand`)
    (set `self.status` "NewEnumerator1")
    (`SceneComponent.SetVisibility` (`self.Vive_Control`) true false)
    (set `self.JustReleased` false))
  (:`Released`
    ;[0 0.7608 1] shoots arrow if placed on bow, else drops arrow from right hand
    (if (`|EnumEquality` (`self.status`) "NewEnumerator2")
      (`self.ArrowShoot`)
      (else
        (`self.ArrowDrop`)))
    (set `self.status` "NewEnumerator0")
    (`PlayerController.PlayDynamicForceFeedback` (`GameplayStatics.GetPlayerController` 0) 0.0 0.0 false false true true)
    (`SceneComponent.SetVisibility` (`self.Vive_Control`) true false)
    (set `self.JustReleased` true)))

(event `Key|MotionController_Left_Trigger`
  (params (Key :type "Key Structure" :default "AnyKey"))
  ;[0 0.7608 1] switches between one and two handed mode - currently not used
)

(event `self.ReceiveTick`
  (params (DeltaSeconds :type "Float (single-precision)"))
  (set `self.deltaSeconds` DeltaSeconds) ; used for timers
  (`|ExecutionSequence`
    (:`then_0`
      ;[0 0.7608 1] attaches arrow to bow when hands are close
      (if (and (`|EnumEquality` (`self.status`) "NewEnumerator1") (< (`self.getDistanceOfHands`) 28.0))
        (set `self.status` "NewEnumerator2")
        (`self.ArrowAttachToBow`)))
    (:`then_1`
      ;[0 0.7608 1] updates bow string and arrow position when arrow is placed
      (if (`|EnumEquality` (`self.status`) "NewEnumerator2")
        (if (`self.TwoHandMode`)
          (`self.BowRotate`))
        (`self.ArrowUpdatePosition`)))))

(event `arrowTrace`
  ;[0 0.7608 1] arrow trace methode. Schiet herhaaldelijk een " nep arrow"
  (bind _returnvalue (`|SpawnActorFromClass` "/Game/MigratedContent_Archery/Vive/Blueprints/BP_ArrowTrace.BP_ArrowTrace_C" (`self.arrow_transform`) "AlwaysSpawn" "OverrideRootScale"))
  (bind _output_get (set `self.traceArrow` _returnvalue))
  (bind _staticmesh (`/Game/MigratedContent_Archery/Vive/Blueprints/BP_ArrowTrace.StaticMesh` _output_get))
  (`SceneComponent.K2_AttachTo` _staticmesh (`/Game/MigratedContent_Archery/Vive/Blueprints/BP_Bow.attachArrowPoint` (`self.bow`)) "None" "SnapToTarget" false)
  (`SceneComponent.DetachFromParent` _staticmesh true false)
  (`ActorComponent.SetActive` (`/Game/MigratedContent_Archery/Vive/Blueprints/BP_ArrowTrace.ProjectileMovement` (`self.traceArrow`)) true false)
  (set `MovementComponent.Velocity` (* (`KismetMathLibrary.GreaterGreater_VectorRotator` (1.0 0.0 0.0) (`SceneComponent.K2_GetComponentRotation` (`/Game/MigratedContent_Archery/Vive/Blueprints/BP_Bow.ForwardArrow` (`self.bow`)))) (`KismetMathLibrary.MapRangeClamped` (`self.getDistanceOfHands`) 10.0 90.0 1000.0 2000.0)) (`/Game/MigratedContent_Archery/Vive/Blueprints/BP_ArrowTrace.ProjectileMovement` (`self.traceArrow`)))
  (`KismetSystemLibrary.Delay` 0.5)
  (`self.K2_DestroyActor` (`self.traceArrow`)))

(event `ArrowDrop`
  (bind _grabbedarrow (`self.grabbedArrow`))
  ;[0 0.7608 1] Arrow drop function
  (`SceneComponent.DetachFromParent` (`/Game/MigratedContent_Archery/Vive/Blueprints/BP_Arrow2.StaticMesh` (`self.grabbedArrow`)) false true)
  (`self.SetActorEnableCollision` _grabbedarrow true)
  (`PrimitiveComponent.SetSimulatePhysics` (`/Game/MigratedContent_Archery/Vive/Blueprints/BP_Arrow2.StaticMesh` _grabbedarrow) true))

(event `ArrowShoot`
  ;[0 0.7608 1] shoot function
  (`GameplayStatics.PlaySound2D` "/Game/MigratedContent_Archery/Vive/Sounds/ArrowSizzleBysHeav_FS036706.ArrowSizzleBysHeav_FS036706")
  (`SceneComponent.DetachFromParent` (`/Game/MigratedContent_Archery/Vive/Blueprints/BP_Arrow2.StaticMesh` (`self.grabbedArrow`)) true false)
  (if (`/Game/MigratedContent_Archery/Vive/Blueprints/BP_Arrow2.isSuperArrow` (`self.grabbedArrow`))
    (`BoxComponent.SetBoxExtent` (`/Game/MigratedContent_Archery/Vive/Blueprints/BP_Arrow2.Box` (`self.grabbedArrow`)) (1500.0 1500.0 0.0) true) ; bigger hitbox when super arrow
    (`SceneComponent.SetWorldScale3D` (`/Game/MigratedContent_Archery/Vive/Blueprints/BP_Arrow2.traceParticle` (`self.grabbedArrow`)) (3.0 3.0 3.0)) ; super particle!
    (set `self.comboCounter` 0) ; reset combo counter to restart chain after super arrow is shot
    (set `ProjectileMovementComponent.ProjectileGravityScale` 0.0 (`/Game/MigratedContent_Archery/Vive/Blueprints/BP_Arrow2.ProjectileMovement` (`self.grabbedArrow`))) ; makes super arrow go in straight line
  )
  (`ActorComponent.SetActive` (`/Game/MigratedContent_Archery/Vive/Blueprints/BP_Arrow2.ProjectileMovement` (`self.grabbedArrow`)) true false)
  (set `MovementComponent.Velocity` (* (`KismetMathLibrary.GreaterGreater_VectorRotator` (1.0 0.0 0.0) (`SceneComponent.K2_GetComponentRotation` (`/Game/MigratedContent_Archery/Vive/Blueprints/BP_Bow.ForwardArrow` (`self.bow`)))) (`KismetMathLibrary.MapRangeClamped` (`self.getDistanceOfHands`) 10.0 90.0 1000.0 2000.0)) (`/Game/MigratedContent_Archery/Vive/Blueprints/BP_Arrow2.ProjectileMovement` (`self.grabbedArrow`)))
  (set `/Game/MigratedContent_Archery/Vive/Blueprints/BP_Arrow2.isShot` true (`self.grabbedArrow`)))

(event `ArrowAttachToBow`
  ;[0 0.7608 1] attaches arrow to bow
  (`SceneComponent.K2_AttachTo` (`/Game/MigratedContent_Archery/Vive/Blueprints/BP_Arrow2.StaticMesh` (`self.grabbedArrow`)) (`/Game/MigratedContent_Archery/Vive/Blueprints/BP_Bow.attachArrowPoint` (`self.bow`)) "None" "SnapToTarget" false))

(event `ArrowSpawnAndAttachToRightHand`
  ;[0 0.7608 1] spawns arrow in right hand when trigger is pressed
  (bind _returnvalue (`|SpawnActorFromClass` "/Game/MigratedContent_Archery/Vive/Blueprints/BP_Arrow2.BP_Arrow2_C" (`self.arrow_transform`) "Undefined" "OverrideRootScale"))
  (bind _output_get (set `self.grabbedArrow` _returnvalue))
  (`self.SetActorEnableCollision` _output_get true)
  (`SceneComponent.K2_AttachTo` (`/Game/MigratedContent_Archery/Vive/Blueprints/BP_Arrow2.StaticMesh` (`self.grabbedArrow`)) (`self.Right_Hand_Controller`) "None" "KeepRelativeOffset" true))

(event `ArrowUpdatePosition`
  (bind _grabbedarrow (`self.grabbedArrow`))
  (bind _grabbedarrow_2 (`self.grabbedArrow`))
  (bind _returnvalue (`KismetMathLibrary.MapRangeClamped` (`self.getDistanceOfHands`) 10.0 90.0 30.0 70.0))
  (bind (_relativelocation_x _relativelocation_y _relativelocation_z) (`KismetMathLibrary.BreakVector` (`SceneComponent.RelativeLocation` (`/Game/MigratedContent_Archery/Vive/Blueprints/BP_Bow.attachArrowPoint` (`self.bow`)))))
  ;[0 0.7608 1] updates arrow and string position when arrow is placed on bow
  (`SceneComponent.K2_SetRelativeLocation` (`/Game/MigratedContent_Archery/Vive/Blueprints/BP_Bow.attachArrowPoint` (`self.bow`)) (`KismetMathLibrary.MakeVector` _returnvalue _relativelocation_y _relativelocation_z) false false)
  (`|ExecutionSequence`
    (:`then_0`
      (if (> _returnvalue 40.0)
        ;;[1 1 1] super arrow when string pulled for 2 seconds
        (set `self.chargeTimer` (+ (`self.chargeTimer`) (`self.deltaSeconds`)))
        (if (> (`self.chargeTimer`) 2.0)
          (set `/Game/MigratedContent_Archery/Vive/Blueprints/BP_Arrow2.isSuperArrow` true _grabbedarrow_2)
          (`ActorComponent.Activate` (`/Game/MigratedContent_Archery/Vive/Blueprints/BP_Arrow2.traceParticle` _grabbedarrow_2) false))
        (else
          ;;[1 1 1] reset arrow charge
          (set `self.chargeTimer` 0.0)
          (set `/Game/MigratedContent_Archery/Vive/Blueprints/BP_Arrow2.isSuperArrow` false _grabbedarrow)
          (`ActorComponent.Deactivate` (`/Game/MigratedContent_Archery/Vive/Blueprints/BP_Arrow2.traceParticle` _grabbedarrow)))))
    (:`then_1`
      (`PlayerController.PlayDynamicForceFeedback` (`GameplayStatics.GetPlayerController` 0) (`KismetMathLibrary.MapRangeClamped` (`self.getDistanceOfHands`) 10.0 90.0 0.1 0.5) 0.05 false false true true))
    (:`then_2`
      (set `self.strength` (- _returnvalue 30.0)))))

(event `BowSpawnAndAttachToLeftHand`
  ;[0 0.7608 1] spawns bow in left hand on begin play
  (bind _returnvalue (`|SpawnActorFromClass` "/Game/MigratedContent_Archery/Vive/Blueprints/BP_Bow.BP_Bow_C" (`self.bow_transform`) "Undefined" "OverrideRootScale"))
  (bind _output_get (set `self.bow` _returnvalue))
  (`self.K2_AttachRootComponentTo` _output_get (`self.Left_Hand_Controller`) "None" "KeepRelativeOffset" true))

(event `ToggleMode`
  ;[0 0.7608 1] switches between one and two handed mode, currently only one handed mode is used
  (set `self.TwoHandMode` (not (`self.TwoHandMode`)))
  (`self.BowResetRotation`))

(event `BowResetRotation`
  ;[0 0.7608 1] used for two handed mode, rotates bow depending on left controller position
  (`self.K2_SetActorRotation` (`self.bow`) (`SceneComponent.K2_GetComponentRotation` (`self.Left_Hand_Controller`)) false))

(event `BowRotate`
  ;[0 0.7608 1] used for two handed mode, rotates bow depending on left controller position
  (`self.K2_SetActorRotation` (`self.bow`) (`KismetMathLibrary.MakeRotator` (.roll (`KismetMathLibrary.Conv_VectorToRotator` (`KismetMathLibrary.GetDirectionVector` (`SceneComponent.K2_GetComponentLocation` (`self.Right_Hand_Controller`)) (`SceneComponent.K2_GetComponentLocation` (`self.Left_Hand_Controller`))))) (+ (.pitch (`KismetMathLibrary.Conv_VectorToRotator` (`KismetMathLibrary.GetDirectionVector` (`SceneComponent.K2_GetComponentLocation` (`self.Right_Hand_Controller`)) (`SceneComponent.K2_GetComponentLocation` (`self.Left_Hand_Controller`))))) 90.0) (.yaw (`KismetMathLibrary.Conv_VectorToRotator` (`KismetMathLibrary.GetDirectionVector` (`SceneComponent.K2_GetComponentLocation` (`self.Right_Hand_Controller`)) (`SceneComponent.K2_GetComponentLocation` (`self.Left_Hand_Controller`)))))) false))

(fn `getDistanceOfHands`
  (returns (ReturnValue :type "Float (double-precision)"))
  (return (`KismetMathLibrary.VSize` (- (`SceneComponent.K2_GetComponentLocation` (`self.Right_Hand_Controller`)) (`SceneComponent.K2_GetComponentLocation` (`self.Left_Hand_Controller`))))))

(fn `UserConstructionScript`)