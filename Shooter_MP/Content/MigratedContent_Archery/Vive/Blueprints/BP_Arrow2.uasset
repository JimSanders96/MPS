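; BP_Arrow2 is an archery arrow projectile that can be lit on fire and leaves flames on enemies it hits.
; Its Box overlap swaps the trail for a fire particle on touching bp_flame, or spawns flames at the box on hitting bp_enemy, whether lit or not.
; Tick shows the trail while IsShot and unlit, then clears it and destroys the arrow after a delay once ProjectileMovement velocity reaches zero.
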(event `self.Box.OnComponentBeginOverlap`
  (params (OverlappedComponent :type "PrimitiveComponent Object Reference") (OtherActor :type "Actor Object Reference") (OtherComp :type "PrimitiveComponent Object Reference") (OtherBodyIndex :type Integer) (bFromSweep :type Boolean) (SweepResult :type "HitResult Structure (by ref)"))
  ;[0 0.7608 1] activates fire particle when arrow is held in fire
  (cast `/Game/MigratedContent_Archery/Vive/Blueprints/bp_flame` OtherActor
    (:`then`
      (`ActorComponent.Activate` (`self.fireParticle`) false)
      (`ActorComponent.Deactivate` (`self.traceParticle`))
      (set `self.onFire?` true))
    (:`CastFailed`
      ;[0 0.7608 1] sets enemy on fire when hit by arrow
      (cast `/Game/MigratedContent_Archery/Vive/Blueprints/bp_enemy` OtherActor)
      (`GameplayStatics.SpawnEmitterAtLocation` "/Game/MigratedContent_Archery/ExampleContent/Blueprint_Communication/Effects/P_Flames.P_Flames" (`SceneComponent.K2_GetComponentLocation` (`self.Box`))))))

(event `self.ReceiveTick`
  (params (DeltaSeconds :type "Float (single-precision)"))
  ;[0 0.7608 1] when arrow shot and not on fire, activates shot particle
  (if (`self.isShot`)
    (if (not (`self.onFire?`))
      (`ActorComponent.Activate` (`self.traceParticle`) false))
    ;[0 0.7608 1] deactivates arrow when it stops moving
    (if (== (`MovementComponent.Velocity` (`self.ProjectileMovement`)) (0.0 0.0 0.0))
      (`ActorComponent.Deactivate` (`self.traceParticle`))
      (set `self.isShot` false)
      ;[0 0.7608 1] destroys arrow after it stops moving
      (`KismetSystemLibrary.Delay` 10.0)
      (`self.K2_DestroyActor`))))

(fn `UserConstructionScript`)